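; BP_AI is a simple AI pawn that chases pawns it sees and can be killed by damage.
; PawnSensing feeds each seen pawn into AIMoveTo as the target actor.
; TakeDmg prints the current HP, subtracts a fixed amount, and destroys the actor when HP is exactly zero, checked before and after the subtraction.
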(event OnSeePawn(PawnSensing)
  (params (Pawn :type Pawn%20Object%20Reference))
  (AI|AIMoveTo self "0, 0, 0" Pawn 5.0 false))

(event Custom|TakeDmg
  (bind _self self)
  (Development|PrintString (Utilities|String|ToString(Float) (Variables|Default|GetHP)))
  (if (== (Variables|Default|GetHP) 0.0)
    (Actor|DestroyActor _self)
    (else
      (bind _output_get (Variables|Default|SetHP (- (Variables|Default|GetHP) 25.0)))
      (if (== _output_get 0.0)
        (Actor|DestroyActor _self)))))

(fn ConstructionScript)