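; Player character Blueprint that handles movement, mouse turning, shooting and a play-time counter.
; Movement follows control rotation and mouse X adds yaw, while the look up/down axis is left disconnected from its pitch input.
; Left click spawns a scaled-down BP_Bullet at ProjectileSpawnPoint.
; Tick runs through a one-second Delay as a makeshift timer, advancing Seconds and Minutes until Ending is set.
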(event EventTick
  (params (DeltaSeconds :type Float%20%28single-precision%29))
  (Utilities|FlowControl|Delay 1.0)
  (if (not (Variables|Default|Getending))
    (Variables|Default|SetSeconds (+ (Variables|Default|GetSeconds) 1))
    (if (> (Variables|Default|GetSeconds) 59)
      (Variables|Default|SetMinutes (+ (Variables|Default|GetMinutes) 1))
      (Variables|Default|SetSeconds 0))))

(event Input|AxisEvents|InputAxisMoveForward/Backward
  (params (AxisValue :type Float%20%28single-precision%29))
  (Pawn|Input|AddMovementInput (Math|Vector|GetForwardVector (Math|Rotator|MakeRotator 0.0 0.0 (.yaw (Pawn|GetControlRotation :!class /Script/Engine.Pawn)))) AxisValue false))

(event Input|AxisEvents|InputAxisMoveRight/Left
  (params (AxisValue :type Float%20%28single-precision%29))
  (bind _returnvalue (Pawn|GetControlRotation :!class /Script/Engine.Pawn))
  (Pawn|Input|AddMovementInput (Math|Vector|GetRightVector (Math|Rotator|MakeRotator (.roll _returnvalue) 0.0 (.yaw _returnvalue))) AxisValue false))

(event Input|AxisEvents|InputAxisTurnRight/LeftMouse
  (params (AxisValue :type Float%20%28single-precision%29))
  (Pawn|Input|AddControllerYawInput AxisValue))

(event Input|AxisEvents|InputAxisLookUp/DownMouse
  (params (AxisValue :type Float%20%28single-precision%29)))

(event Input|MouseEvents|LeftMouseButton
  (params (Key :type Key%20Structure :default "None"))
  (bind _projectilespawnpoint (Variables|Default|GetProjectileSpawnPoint))
  (bind _returnvalue (Transformation|GetWorldTransform _projectilespawnpoint))
  (:Pressed
    (Game|SpawnActorfromClass "/Game/Blueprints/BP_Bullet.BP_Bullet_C" (Math|Transform|MakeTransform (.location _returnvalue) (.rotation _returnvalue) "0.100000,0.100000,0.100000") "Undefined" 0 0)))

(fn ConstructionScript)