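; BP_Enemy is an enemy actor Blueprint with health and projectile shooting functions.
; Shoot spawns a scaled-down BP_Bullet at ProjectileSpawnPoint and plays a 2D sound.
; TakeDamage destroys the actor when Health is zero or below, but its Health subtraction is disconnected and never runs.
; AnyDamage and ShootingLoop are empty, and nothing here calls Shoot or TakeDamage.
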(event Game|Damage|EventAnyDamage
  (params (Damage :type Float%20%28single-precision%29) (DamageType :type Damage%20Type%20Object%20Reference) (InstigatedBy :type Controller%20Object%20Reference) (DamageCauser :type Actor%20Object%20Reference)))

(fn ConstructionScript)

(fn TakeDamage
  (params (Damage :type Float%20%28double-precision%29))
  (if (<= (Variables|Default|GetHealth) 0.0)
    (Actor|DestroyActor)))

(fn Shoot
  (bind _projectilespawnpoint (Variables|Default|GetProjectileSpawnPoint))
  (bind _returnvalue (Transformation|GetWorldTransform _projectilespawnpoint))
  (Game|SpawnActorfromClass "/Game/Blueprints/BP_Bullet.BP_Bullet_C" (Math|Transform|MakeTransform (.location _returnvalue) (.rotation _returnvalue) "0.050000,0.050000,0.050000") "Undefined" 0 0)
  (Audio|PlaySound2D 0 1.0 1.0 0.0 0 0))

(fn ShootingLoop)